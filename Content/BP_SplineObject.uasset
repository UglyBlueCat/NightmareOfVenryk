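; BP_SplineObject is an actor that travels along a referenced spline once play begins, with a configurable mesh set in the construction script.
; A timeline, with its play rate set to the inverse of TimeToComplete, drives the movement.
; Each update maps the timeline track to a distance along the spline's length and applies that point's world location and rotation to the actor.
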(event `self.ReceiveBeginPlay`
  (`self.Move Object`))

(event `Move Object`
  (bind _spline (`/Game/BP_SplinePath.Spline` (`self.Spline to Follow`)))
  (`TimelineComponent.SetPlayRate` (`self.T_Move`) (/ 1.0 (`self.Time to Complete`)))
  (bind (_direction _move_track) (`Timeline|T_Move`)
    (:`Update`
      (bind _returnvalue (`KismetMathLibrary.Lerp` 0.0 (`SplineComponent.GetSplineLength` _spline) _move_track))
      (`self.K2_SetActorLocationAndRotation` (`SplineComponent.GetLocationAtDistanceAlongSpline` _spline _returnvalue "World") (`SplineComponent.GetRotationAtDistanceAlongSpline` _spline _returnvalue "World")))))

(fn `UserConstructionScript`
  (`StaticMeshComponent.SetStaticMesh` (`self.Cube`) (`self.Object Mesh`)))